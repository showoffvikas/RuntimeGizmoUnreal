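; BP_Gizmo is a gizmo Blueprint that switches between six directional cameras: top, down, front, back and two sides.
; BeginPlay gathers the camera components into an ordered array.
; SetCam1 takes an index, loops over the array and activates only the matching camera, deactivating all the others.
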(event EventBeginPlay
  (Variables|Default|SetCamArray (Utilities|Array|MakeArray (Variables|Default|GetTopCam) (Variables|Default|GetDownCam) (Variables|Default|GetFrontCam) (Variables|Default|GetBackCam) (Variables|Default|GetSide1Cam) (Variables|Default|GetSide2Cam))))

(fn ConstructionScript)

(fn SetCam1
  (params (CurrCamIndx :type Integer))
  (for (_array_element _array_index) (Variables|Default|GetCamArray)
    (if (== CurrCamIndx _array_index)
      (Components|Activation|SetActive _array_element true false)
      (else
        (Components|Activation|SetActive _array_element false false)))))